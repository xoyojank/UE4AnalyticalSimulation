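; BP_Ghost is a short-lived actor with a sphere mesh that destroys itself after its lifetime, fading out through its material.
; On BeginPlay it creates a dynamic material instance on the sphere and passes it the spawn time, lifetime and fade time.
; The Blueprint only waits and destroys the actor, leaving any time-based fade to the material rather than updating it on Tick.
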(event `self.ReceiveBeginPlay`
  (bind _returnvalue (`PrimitiveComponent.CreateDynamicMaterialInstance` (`self.Sphere`) 0 null "None"))
  (bind _output_get (set `self.MaterialInstance` _returnvalue))
  (`MaterialInstanceDynamic.SetScalarParameterValue` _output_get "SpawnTime" (`GameplayStatics.GetTimeSeconds`))
  (`MaterialInstanceDynamic.SetScalarParameterValue` _output_get "LifeTime" (`self.LifeTime`))
  (`MaterialInstanceDynamic.SetScalarParameterValue` _output_get "FadeTime" (`self.FadeTime`))
  (`KismetSystemLibrary.Delay` (`self.LifeTime`))
  (`self.K2_DestroyActor`))

(fn `UserConstructionScript`)